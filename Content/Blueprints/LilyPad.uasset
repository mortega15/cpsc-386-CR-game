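; LilyPad is an actor that tells the player when it is standing on the pad.
; Overlap begin and end on its Box set IsOnLilyPad on BP_Player to true or false.
; Tick polls the player's Restarting flag and, when set, destroys only the LilyPad component, guarded by LilyPadDestroyed so it runs once.
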(event OnComponentBeginOverlap(Box)
  (params (OverlappedComponent :type Primitive%20Component%20Object%20Reference) (OtherActor :type Actor%20Object%20Reference) (OtherComp :type Primitive%20Component%20Object%20Reference) (OtherBodyIndex :type Integer) (bFromSweep :type Boolean) (SweepResult :type Hit%20Result%20Structure%20%28by%20ref%29))
  (bind _asbp_player (Utilities|Casting|CastToBP_Player OtherActor))
  (Variables|/Game/Blueprints/BP_Player.BP_Player_C|SetIsOnLilyPad _asbp_player true))

(event OnComponentEndOverlap(Box)
  (params (OverlappedComponent :type Primitive%20Component%20Object%20Reference) (OtherActor :type Actor%20Object%20Reference) (OtherComp :type Primitive%20Component%20Object%20Reference) (OtherBodyIndex :type Integer))
  (bind _asbp_player (Utilities|Casting|CastToBP_Player OtherActor))
  (Variables|/Game/Blueprints/BP_Player.BP_Player_C|SetIsOnLilyPad _asbp_player false))

(event EventBeginPlay)

(event Collision|EventActorBeginOverlap
  (params (OtherActor :type Actor%20Object%20Reference)))

(event EventTick
  (params (DeltaSeconds :type Float%20%28single-precision%29))
  (if (not (Variables|Default|GetLilyPadDestroyed))
    (bind _asbp_player (Utilities|Casting|CastToBP_Player (Game|GetPlayerCharacter 0)))
    (if (Variables|/Game/Blueprints/BP_Player.BP_Player_C|GetRestarting _asbp_player)
      (Components|DestroyComponent (Variables|Default|GetLilyPad))
      (Variables|Default|SetLilyPadDestroyed true))))

(fn ConstructionScript)